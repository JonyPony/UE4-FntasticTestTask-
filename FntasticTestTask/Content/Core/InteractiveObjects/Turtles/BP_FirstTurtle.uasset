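; Interactive turtle that, once activated, travels from a start transform to an end transform, then disappears in a shower of coins.
; Activation spawns an attached coin burst, starts a 2D footstep sound and plays a timeline that lerps the skeletal mesh's world position and rotation, holding the starting Z.
; When the timeline finishes it ends the interaction; the end event spawns the coin shower, destroys the actor and stops the audio.
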(event `self.OnActivatedForInteract`
  (params (InstigatedBy :type "Actor Object Reference") (InstigatorInteractionComponent :type "FTT_InteractionComponent Object Reference"))
  (bind _turtlestarttransform (`self.TurtleStartTransform`))
  (`parent.OnActivatedForInteract` InstigatedBy InstigatorInteractionComponent)
  (`NiagaraFunctionLibrary.SpawnSystemAttached` "/Game/VFX/Fx/NiagaraSystems/NS_CoinBurst.NS_CoinBurst" (`self.SkeletalMesh`) "None" (0.0 0.0 0.0) (struct) "KeepRelativeOffset" true)
  (bind _returnvalue (`GameplayStatics.CreateSound2D` "/Game/Sound/SFX_TurtleFootstep.SFX_TurtleFootStep" 1.0 1.0 0.0 null))
  (bind _output_get (set `self.AudioComponent` _returnvalue))
  (`AudioComponent.Play` _output_get 0.0)
  (bind (_direction _alpha) (`Timeline|Timeline_0` :`NewTime` 10.0)
    (:`Update`
      (bind _returnvalue_2 (`KismetMathLibrary.TLerp` _turtlestarttransform (`self.TurtleEndTransform`) _alpha))
      (`SceneComponent.K2_SetWorldLocationAndRotation` (`self.SkeletalMesh`) (`KismetMathLibrary.MakeVector` (.x (.location _returnvalue_2)) (.y (.location _returnvalue_2)) (.z (.location _turtlestarttransform))) (.rotation _returnvalue_2) false true))
    (:`Finished`
      (`FTT_InteractionComponent.EndInteractWith` InstigatorInteractionComponent self))))

(event `self.OnEndIntaractWith`
  (params (InteractedActor :type "Actor Object Reference") (InteractionComponent :type "FTT_InteractionComponent Object Reference"))
  (bind (_turtleendtransform_location _turtleendtransform_rotation) (`KismetMathLibrary.BreakTransform` (`self.TurtleEndTransform`)))
  (`parent.OnEndIntaractWith` InteractedActor InteractionComponent)
  (`NiagaraFunctionLibrary.SpawnSystemAtLocation` "/Game/VFX/Fx/NiagaraSystems/NS_Coin_Shower.NS_Coin_Shower" _turtleendtransform_location _turtleendtransform_rotation (3.0 3.0 3.0))
  (`self.K2_DestroyActor`)
  (`AudioComponent.Stop` (`self.AudioComponent`)))

(fn `UserConstructionScript`)