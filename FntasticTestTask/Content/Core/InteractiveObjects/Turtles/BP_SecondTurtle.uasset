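; Interactive turtle that, once activated, travels from a start to an end transform in a stop-and-go rhythm with looping timers and footstep audio.
; The MoveTurtle timeline lerps the mesh's XY and rotation at fixed start height, while alternating timer events pause and resume movement and sound.
; Coin effects mark activation and completion; timeline completion ends the interaction, which plays the finish sound and destroys the actor.
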(event `self.OnActivatedForInteract`
  (params (InstigatedBy :type "Actor Object Reference") (InstigatorInteractionComponent :type "FTT_InteractionComponent Object Reference"))
  (bind _turtlestarttransform (`self.TurtleStartTransform`))
  (set `self.Instigator Interaction Component` InstigatorInteractionComponent)
  (`parent.OnActivatedForInteract` InstigatedBy InstigatorInteractionComponent)
  (`GameplayStatics.PlaySound2D` "/Game/Sound/SFX_TurtleStart.SFX_TurtleStart" 1.0 1.0 0.0 null null)
  (`NiagaraFunctionLibrary.SpawnSystemAttached` "/Game/VFX/Fx/NiagaraSystems/NS_CoinBurst.NS_CoinBurst" (`self.SkeletalMesh`) "None" (0.0 0.0 0.0) (struct) "KeepRelativeOffset" true)
  (bind _returnvalue (`GameplayStatics.CreateSound2D` "/Game/Sound/SFX_TurtleFootstep.SFX_TurtleFootStep" 1.0 1.0 0.0 null))
  (bind _output_get (set `self.AudioComponent` _returnvalue))
  (`AudioComponent.Play` _output_get 0.0)
  (`KismetSystemLibrary.K2_SetTimerDelegate` (delegate `Stop`) 1.0 :!label _label)
  (`AudioComponent.SetPaused` (`self.AudioComponent`) false)
  (bind (_direction _alpha) (`Timeline|MoveTurtle` :`NewTime` 10.0 :!label _label_2)
    (:`Update`
      (bind _returnvalue_2 (`KismetMathLibrary.TLerp` _turtlestarttransform (`self.TurtleEndTransform`) _alpha))
      (`SceneComponent.K2_SetWorldLocationAndRotation` (`self.SkeletalMesh`) (`KismetMathLibrary.MakeVector` (.x (.location _returnvalue_2)) (.y (.location _returnvalue_2)) (.z (.location _turtlestarttransform))) (.rotation _returnvalue_2) false true))
    (:`Finished`
      (`FTT_InteractionComponent.EndInteractWith` (`self.Instigator Interaction Component`) self))))

(event `Stop`
  (`|ExecutionSequence`
    (:`then_0`
      (`AudioComponent.SetPaused` (`self.AudioComponent`) true)
      (goto _label_2 :!via `Stop`))
    (:`then_1`
      (`KismetSystemLibrary.K2_SetTimerDelegate` (delegate `Play`) 0.5))))

(event `Play`
  (`|ExecutionSequence`
    (:`then_0`
      (goto _label))
    (:`then_1`
      (goto _label_2))))

(event `self.OnEndIntaractWith`
  (params (InteractedActor :type "Actor Object Reference") (InteractionComponent :type "FTT_InteractionComponent Object Reference"))
  (bind (_turtleendtransform_location _turtleendtransform_rotation) (`KismetMathLibrary.BreakTransform` (`self.TurtleEndTransform`)))
  (`parent.OnEndIntaractWith` InteractedActor InteractionComponent)
  (`GameplayStatics.PlaySound2D` "/Game/Sound/SFX_TurtleFinish.SFX_TurtleFinish" 1.0 1.0 0.0 null null)
  (`NiagaraFunctionLibrary.SpawnSystemAtLocation` "/Game/VFX/Fx/NiagaraSystems/NS_Coin_Shower.NS_Coin_Shower" _turtleendtransform_location _turtleendtransform_rotation (3.0 3.0 3.0) true true "AutoRelease")
  (`AudioComponent.Stop` (`self.AudioComponent`))
  (`self.K2_DestroyActor`))

(fn `UserConstructionScript`)