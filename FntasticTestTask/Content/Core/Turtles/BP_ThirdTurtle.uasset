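; Interactable turtle that, when activated, bursts coins and travels to TurtleEndLocation while a footstep sound plays.
; A timeline lerps the skeletal mesh's XY and rotation toward the target, holding the starting Z.
; Looping timers alternate the timeline between forward play and shorter reversals, creating a back-and-forth advance.
; Timeline completion ends the interaction; the end-interaction handler spawns a coin shower at the target, destroys the actor and stops the sound.
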(event `self.OnActivatedForInteract`
  (params (InstigatedBy :type "Actor Object Reference") (InstigatorInteractionComponent :type "FTT_InteractionComponent Object Reference"))
  (bind _newvar_1 (`self.NewVar_1`))
  (set `self.Instigator Interaction Component` InstigatorInteractionComponent)
  (`parent.OnActivatedForInteract` InstigatedBy InstigatorInteractionComponent)
  (set `self.NewVar_1` (`self.GetTransform`))
  (`NiagaraFunctionLibrary.SpawnSystemAttached` "/Game/VFX/Fx/NiagaraSystems/NS_CoinBurst.NS_CoinBurst" (`self.SkeletalMesh`) "None" (0.0 0.0 0.0) (struct) "KeepRelativeOffset" true)
  (bind _returnvalue (`GameplayStatics.CreateSound2D` "/Game/Sound/SFX_TurtleFootstep.SFX_TurtleFootStep" 1.0 1.0 0.0 null))
  (bind _output_get (set `self.NewVar_0` _returnvalue))
  (`AudioComponent.Play` _output_get 0.0)
  (`KismetSystemLibrary.K2_SetTimerDelegate` (delegate `Move`) 1.0 :!label _label)
  (bind (_direction _newtrack_0) (`Timeline|Timeline_0` :`NewTime` 10.0 :!label _label_2)
    (:`Update`
      (bind _returnvalue_2 (`KismetMathLibrary.TLerp` _newvar_1 (`self.TurtleEndLocation`) _newtrack_0))
      (`SceneComponent.K2_SetWorldLocationAndRotation` (`self.SkeletalMesh`) (`KismetMathLibrary.MakeVector` (.x (.location _returnvalue_2)) (.y (.location _returnvalue_2)) (.z (.location _newvar_1))) (.rotation _returnvalue_2) false true))
    (:`Finished`
      (`FTT_InteractionComponent.EndInteractWith` (`self.Instigator Interaction Component`) self))))

(event `Move`
  (`|ExecutionSequence`
    (:`then_0`
      (goto _label_2 :!via `Reverse`))
    (:`then_1`
      (`KismetSystemLibrary.K2_SetTimerDelegate` (delegate `CustomEvent_0`) 0.5))))

(event `self.OnEndIntaractWith`
  (params (InteractedActor :type "Actor Object Reference") (InteractionComponent :type "FTT_InteractionComponent Object Reference"))
  (bind (_turtleendlocation_location _turtleendlocation_rotation) (`KismetMathLibrary.BreakTransform` (`self.TurtleEndLocation`)))
  (`parent.OnEndIntaractWith` InteractedActor InteractionComponent)
  (`NiagaraFunctionLibrary.SpawnSystemAtLocation` "/Game/VFX/Fx/NiagaraSystems/NS_Coin_Shower.NS_Coin_Shower" _turtleendlocation_location _turtleendlocation_rotation (3.0 3.0 3.0))
  (`self.K2_DestroyActor`)
  (`AudioComponent.Stop` (`self.NewVar_0`)))

(event `CustomEvent_0`
  (`|ExecutionSequence`
    (:`then_0`
      (goto _label_2))
    (:`then_1`
      (goto _label))))

(fn `UserConstructionScript`)