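; BP_FirstTurtle is an interactable turtle that travels to an end point and pays off with a coin shower.
; Activation plays a coin burst and footstep sound, then slides the skeletal mesh toward TurtleEndLocation with a timed latent MoveComponentTo.
; When the move completes, it ends the interaction itself.
; The end-interact event spawns the coin shower at the end point, destroys the actor and stops the sound.
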(event `self.OnActivatedForInteract`
  (params (InstigatedBy :type "Actor Object Reference") (InstigatorInteractionComponent :type "FTT_InteractionComponent Object Reference"))
  (bind _turtleendlocation (`self.TurtleEndLocation`))
  (`parent.OnActivatedForInteract` InstigatedBy InstigatorInteractionComponent)
  (`NiagaraFunctionLibrary.SpawnSystemAttached` "/Game/VFX/Fx/NiagaraSystems/NS_CoinBurst.NS_CoinBurst" (`self.SkeletalMesh`) "None" (0.0 0.0 0.0) (struct) "KeepRelativeOffset" true)
  (bind _returnvalue (`GameplayStatics.CreateSound2D` "/Game/Sound/SFX_TurtleFootstep.SFX_TurtleFootStep" 1.0 1.0 0.0 null))
  (bind _output_get (set `self.NewVar_0` _returnvalue))
  (`AudioComponent.Play` _output_get 0.0)
  (`KismetSystemLibrary.MoveComponentTo` (`self.SkeletalMesh`) (`KismetMathLibrary.MakeVector` (.x (.location _turtleendlocation)) (.y (.location _turtleendlocation))) (`SceneComponent.K2_GetComponentRotation` (`self.SkeletalMesh`)) false false 10.0 true)
  (`FTT_InteractionComponent.EndInteractWith` InstigatorInteractionComponent self))

(event `self.OnEndIntaractWith`
  (params (InteractedActor :type "Actor Object Reference") (InteractionComponent :type "FTT_InteractionComponent Object Reference"))
  (bind (_turtleendlocation_location _turtleendlocation_rotation) (`KismetMathLibrary.BreakTransform` (`self.TurtleEndLocation`)))
  (`parent.OnEndIntaractWith` InteractedActor InteractionComponent)
  (`NiagaraFunctionLibrary.SpawnSystemAtLocation` "/Game/VFX/Fx/NiagaraSystems/NS_Coin_Shower.NS_Coin_Shower" _turtleendlocation_location _turtleendlocation_rotation (3.0 3.0 3.0))
  (`self.K2_DestroyActor`)
  (`AudioComponent.Stop` (`self.NewVar_0`)))

(fn `UserConstructionScript`)